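; BP_WizardAdventureGameMode is the game mode that owns the on-screen UI for the wizard adventure game.
; On BeginPlay it creates the in-game info widget, adds it to the viewport and hands it to the player's BP_Wizard pawn.
; UpdateMonster pushes the current monster count to that widget.
; GameClear and GameOver each show their result widget after a short delay.
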(event `self.ReceiveBeginPlay`
  (bind _returnvalue (`|CreateWidget` "/Game/Game/Blueprints/Widgets/WGB_InGameInfo.WGB_InGameInfo_C"))
  (bind _output_get (set `self.WGB_InGameInfo` _returnvalue))
  (`UserWidget.AddToViewport` _output_get 0)
  (bind _asbp_wizard (cast `/Game/Game/Blueprints/Actors/BP_Wizard` (`GameplayStatics.GetPlayerPawn` 0)))
  (set `/Game/Game/Blueprints/Actors/BP_Wizard.WGBInGameInfo` _output_get _asbp_wizard))

(event `self.UpdateMonster`
  (params (NowMonsterCount :type Integer))
  (`/Game/Game/Blueprints/Widgets/WGB_InGameInfo.SetMonsterCountText` (`self.WGB_InGameInfo`) NowMonsterCount))

(event `self.GameClear`
  (`KismetSystemLibrary.Delay` 1.0)
  (bind _returnvalue (`|CreateWidget` "/Game/Game/Blueprints/Widgets/WGB_GameClear.WGB_GameClear_C"))
  (`UserWidget.AddToViewport` _returnvalue 0))

(event `self.GameOver`
  (`KismetSystemLibrary.Delay` 1.0)
  (bind _returnvalue (`|CreateWidget` "/Game/Game/Blueprints/Widgets/WGB_GameOver.WGB_GameOver_C"))
  (`UserWidget.AddToViewport` _returnvalue 0))

(fn `UserConstructionScript`)